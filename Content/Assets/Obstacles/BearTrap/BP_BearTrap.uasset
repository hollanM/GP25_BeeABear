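; Bear trap obstacle that snaps shut on the player character and holds them in place by disabling input.
; A box overlap while the trap is set plays the TrapClosing timeline, rotating both clamps, then restores input after a short delay.
; The same timeline then plays in reverse to reopen the jaws, with a TrapResetting flag letting its shared Finished branch re-arm the trap.
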(event `self.Box.OnComponentBeginOverlap`
  (params (OverlappedComponent :type "PrimitiveComponent Object Reference") (OtherActor :type "Actor Object Reference") (OtherComp :type "PrimitiveComponent Object Reference") (OtherBodyIndex :type Integer) (bFromSweep :type Boolean) (SweepResult :type "HitResult Structure (by ref)"))
  (if (== OtherActor (`GameplayStatics.GetPlayerCharacter` 0))
    (if (`self.Trap Set?`)
      (`self.Trap Triggered`))))

(event `Trap Triggered`
  (set `self.Trap Set?` false)
  (`self.DisableInput` (`GameplayStatics.GetPlayerCharacter` 0) (`GameplayStatics.GetPlayerController` 0))
  (set `self.player stuck` true)
  (bind (_direction _trap_rotation) (`Timeline|trap closing` :!via `PlayFromStart` :!label _label)
    (:`Update`
      (`SceneComponent.K2_SetRelativeRotation` (`self.trap clamp 1`) (`KismetMathLibrary.RLerp` (struct) (struct :`Roll` -80.0) _trap_rotation) false false)
      (`SceneComponent.K2_SetRelativeRotation` (`self.trap clamp 2`) (`KismetMathLibrary.RLerp` (struct :`Yaw` 179.99) (struct :`Yaw` 179.99 :`Roll` -80.0) _trap_rotation) false false))
    (:`Finished`
      (if (`self.Trap Resetting?`)
        (set `self.Trap Set?` true)
        (set `self.Trap Resetting?` false)
        (else
          (`KismetSystemLibrary.Delay` 1.0)
          (`self.EnableInput` (`GameplayStatics.GetPlayerCharacter` 0) (`GameplayStatics.GetPlayerController` 0))
          (set `self.player stuck` false)
          (`self.Trap Resetting`))))))

(event `Trap Resetting`
  (set `self.Trap Resetting?` true)
  (goto _label :!via `ReverseFromEnd`))

(fn `UserConstructionScript`)