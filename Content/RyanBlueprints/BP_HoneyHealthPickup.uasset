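; BP_HoneyHealthPickup is a honey pickup that heals the player character.
; It caches player 0's BP_ThirdPersonCharacter on BeginPlay and compares it with actors overlapping its Box.
; A player overlap passes a DoOnce, then calls HealPlayer with a fixed amount and destroys the pickup if health is below maximum.
; The DoOnce precedes the health check and is never reset, so touching it at full health leaves it inert.
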(event `self.ReceiveBeginPlay`
  (bind _asbp_third_person_character (cast `/Game/ThirdPerson/Blueprints/BP_ThirdPersonCharacter` (`GameplayStatics.GetPlayerCharacter` 0)))
  (set `self.As BP Third Person Character` _asbp_third_person_character))

(event `self.Box.OnComponentBeginOverlap`
  (params (OverlappedComponent :type "PrimitiveComponent Object Reference") (OtherActor :type "Actor Object Reference") (OtherComp :type "PrimitiveComponent Object Reference") (OtherBodyIndex :type Integer) (bFromSweep :type Boolean) (SweepResult :type "HitResult Structure (by ref)"))
  (bind _as_bp_third_person_character (`self.As BP Third Person Character`))
  (if (== OtherActor (`self.As BP Third Person Character`))
    (`/Engine/EditorBlueprintResources/StandardMacros.DoOnce` false
      (:`Completed`
        (if (< (`/Game/ThirdPerson/Blueprints/BP_ThirdPersonCharacter.Health` _as_bp_third_person_character) (`/Game/ThirdPerson/Blueprints/BP_ThirdPersonCharacter.MaxHealth` _as_bp_third_person_character))
          (`/Game/ThirdPerson/Blueprints/BP_ThirdPersonCharacter.HealPlayer` (`self.As BP Third Person Character`) 20.0)
          (`self.K2_DestroyActor` self))))))

(fn `UserConstructionScript`)