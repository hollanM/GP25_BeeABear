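; BP_BrambleBush is a bramble bush hazard that hurts the player's bear and can be interacted with once for a speed boost.
; Entering the damage box hurts the bear immediately and starts a looping timer that repeats the damage until it leaves.
; A separate interact box shows and hides a hold-to-interact prompt widget, while Interact calls the bear's SpeedBoost through a DoOnce.
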(event `self.ReceiveBeginPlay`
  (bind _asbp_bear (cast `/Game/Graceartstuff/BP_Bear` (`GameplayStatics.GetPlayerCharacter` 0)))
  (set `self.Bear` _asbp_bear)
  (bind _returnvalue (`|CreateWidget` "/Game/RyanWidgets/WBP_InteractHold.WBP_InteractHold_C"))
  (set `self.InteractHoldPrompt` _returnvalue))

(event `self.Box.OnComponentBeginOverlap`
  (params (OverlappedComponent :type "PrimitiveComponent Object Reference") (OtherActor :type "Actor Object Reference") (OtherComp :type "PrimitiveComponent Object Reference") (OtherBodyIndex :type Integer) (bFromSweep :type Boolean) (SweepResult :type "HitResult Structure (by ref)"))
  (if (== OtherActor (`self.Bear`))
    (`GameplayStatics.ApplyDamage` (`self.Bear`) 5.0 null self)
    (bind _returnvalue (`KismetSystemLibrary.K2_SetTimerDelegate` (delegate `BushDamage`) 1.0 true))
    (bind _output_get (set `self.AreaOfDamage` _returnvalue))))

(event `BushDamage`
  (`GameplayStatics.ApplyDamage` (`self.Bear`) 5.0 null self))

(event `self.Box.OnComponentEndOverlap`
  (params (OverlappedComponent :type "PrimitiveComponent Object Reference") (OtherActor :type "Actor Object Reference") (OtherComp :type "PrimitiveComponent Object Reference") (OtherBodyIndex :type Integer))
  (if (== (`self.Bear`) OtherActor)
    (`KismetSystemLibrary.K2_ClearAndInvalidateTimerHandle` (stale `self.Box.OnComponentBeginOverlap` _output_get))))

(event `self.BoxInteract.OnComponentBeginOverlap`
  (params (OverlappedComponent :type "PrimitiveComponent Object Reference") (OtherActor :type "Actor Object Reference") (OtherComp :type "PrimitiveComponent Object Reference") (OtherBodyIndex :type Integer) (bFromSweep :type Boolean) (SweepResult :type "HitResult Structure (by ref)"))
  (if (== OtherActor (`self.Bear`))
    (`UserWidget.AddToViewport` (`self.InteractHoldPrompt`) 0)))

(event `self.BoxInteract.OnComponentEndOverlap`
  (params (OverlappedComponent :type "PrimitiveComponent Object Reference") (OtherActor :type "Actor Object Reference") (OtherComp :type "PrimitiveComponent Object Reference") (OtherBodyIndex :type Integer))
  (if (== (`self.Bear`) OtherActor)
    (`Widget.RemoveFromParent` (`self.InteractHoldPrompt`))))

(event `/Game/RyanBlueprints/I_InteractInterface.Interact`
  (`/Engine/EditorBlueprintResources/StandardMacros.DoOnce` false
    (:`Completed`
      (`/Game/Graceartstuff/BP_Bear.SpeedBoost` (`self.Bear`)))))

(fn `UserConstructionScript`)