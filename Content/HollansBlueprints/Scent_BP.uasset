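; Scent actor with a Niagara ribbon that receives the location of the Cave_BP actor as its CaveLocation parameter.
; On BeginPlay it creates a hold-to-interact widget and passes that cave location to the ribbon.
; An interaction box shows the widget when the player character enters and removes it on exit.
; The custom event ends at a DoOnce with no further action, and a SpawnActor node is left unconnected.
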(event `self.BoxInteract.OnComponentBeginOverlap`
  (params (OverlappedComponent :type "PrimitiveComponent Object Reference") (OtherActor :type "Actor Object Reference") (OtherComp :type "PrimitiveComponent Object Reference") (OtherBodyIndex :type Integer) (bFromSweep :type Boolean) (SweepResult :type "HitResult Structure (by ref)"))
  (if (== OtherActor (`GameplayStatics.GetPlayerCharacter` 0))
    (`UserWidget.AddToViewport` (`self.interactWG`) 0)))

(event `self.BoxInteract.OnComponentEndOverlap`
  (params (OverlappedComponent :type "PrimitiveComponent Object Reference") (OtherActor :type "Actor Object Reference") (OtherComp :type "PrimitiveComponent Object Reference") (OtherBodyIndex :type Integer))
  (if (== (`GameplayStatics.GetPlayerCharacter` 0) OtherActor)
    (`Widget.RemoveFromParent` (`self.interactWG`))))

(event `self.ReceiveBeginPlay`
  (bind _returnvalue (`|CreateWidget` "/Game/RyanWidgets/WBP_InteractHold.WBP_InteractHold_C"))
  (set `self.interactWG` _returnvalue)
  (bind _returnvalue_2 (`GameplayStatics.GetActorOfClass` "/Game/HollansBlueprints/Cave_BP.Cave_BP_C"))
  (`NiagaraComponent.SetVariableVec3` (`self.NS_RibbonBasic`) "CaveLocation" (`self.K2_GetActorLocation` _returnvalue_2)))

(event `CustomEvent`
  (`/Engine/EditorBlueprintResources/StandardMacros.DoOnce` false))

(fn `UserConstructionScript`)