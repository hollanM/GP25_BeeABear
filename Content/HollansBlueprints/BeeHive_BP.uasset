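; Beehive pickup that releases a bee swarm and can heal the player.
; When a third-person character overlaps its collider, it spawns a BeeSwarm_BP at a random navigable point within SpawnRadius.
; If player 0's health is below full, it adds a small uncapped amount and destroys itself; otherwise it remains and can spawn more swarms.
; Honey sound and splash effects are only debug-print placeholders.
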(event `self.BeehiveCollider.OnComponentBeginOverlap`
  (params (OverlappedComponent :type "PrimitiveComponent Object Reference") (OtherActor :type "Actor Object Reference") (OtherComp :type "PrimitiveComponent Object Reference") (OtherBodyIndex :type Integer) (bFromSweep :type Boolean) (SweepResult :type "HitResult Structure (by ref)"))
  (cast `/Game/ThirdPerson/Blueprints/BP_ThirdPersonCharacter` OtherActor
    (:`then`
      (`KismetSystemLibrary.PrintString` "SpawningBees")
      (bind _randomlocation (`NavigationSystemV1.K2_GetRandomLocationInNavigableRadius` (`self.K2_GetActorLocation`) (`self.spawnRadius`) null null))
      (`|SpawnActorFromClass` "/Game/HollansBlueprints/BeeSwarmEnemy/BeeSwarm_BP.BeeSwarm_BP_C" (`KismetMathLibrary.Conv_VectorToTransform` _randomlocation) "AdjustIfPossibleButAlwaysSpawn" "MultiplyWithRoot" null null)
      (bind _asbp_third_person_character (cast `/Game/ThirdPerson/Blueprints/BP_ThirdPersonCharacter` (`GameplayStatics.GetPlayerCharacter` 0)))
      (bind _health (`/Game/ThirdPerson/Blueprints/BP_ThirdPersonCharacter.Health` _asbp_third_person_character))
      (if (< _health 100.0)
        (set `/Game/ThirdPerson/Blueprints/BP_ThirdPersonCharacter.Health` (+ _health 10.0) _asbp_third_person_character)
        (`KismetSystemLibrary.PrintString` "Optional: play honey splat or honey eating sound.           Possible add honey particle splash effect")
        (`self.K2_DestroyActor`)))
    (:`CastFailed`
      (`KismetSystemLibrary.PrintString` "Not the player, No bees are spawning"))))

(fn `UserConstructionScript`)